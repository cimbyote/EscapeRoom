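; Door actor that swings open and closed in response to open and close requests from its OpenDoor member.
; The DoorSwing timeline plays or reverses, feeding its angle track into a yaw rotation combined with the rotation cached at BeginPlay.
; An event track on the same timeline times the door lock sound at the actor's location.
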(event OnOpenRequest(OpenDoor)
  (bind _openangle (Timeline|DoorSwing Play)
    (:Update
      (Transformation|SetActorRotation (Math|Rotator|CombineRotators (Math|Rotator|MakeRotator 0.0 0.0 _openangle) (Variables|Default|GetInitialRotation))))
    (:SoundTiming
      (Audio|PlaySoundatLocation "/Game/Audio/door-lock.door-lock" (Transformation|GetActorLocation) "0, 0, 0" 1.0 1.0 0.0 0 0 0))))

(event OnCloseRequest(OpenDoor)
  (bind _openangle (Timeline|DoorSwing Reverse)
    (:Update
      (Transformation|SetActorRotation (Math|Rotator|CombineRotators (Math|Rotator|MakeRotator 0.0 0.0 _openangle) (Variables|Default|GetInitialRotation))))
    (:SoundTiming
      (Audio|PlaySoundatLocation "/Game/Audio/door-lock.door-lock" (Transformation|GetActorLocation) "0, 0, 0" 1.0 1.0 0.0 0 0 0))))

(event EventBeginPlay
  (Variables|Default|SetInitialRotation (Transformation|GetActorRotation)))

(fn ConstructionScript)